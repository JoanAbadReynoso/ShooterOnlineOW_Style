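; Claymore mine actor that explodes when a BP_Base_Character overlaps its Box trigger.
; The overlap applies full radial damage at the actor's location, ignoring the overlapping character's owner, then draws a debug sphere of the damage radius and spawns an explosion emitter.
; It plays the CompileFailed sound at world origin rather than at the mine, and the actor is not destroyed afterward.
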(event `self.Box.OnComponentBeginOverlap`
  (params (OverlappedComponent :type "PrimitiveComponent Object Reference") (OtherActor :type "Actor Object Reference") (OtherComp :type "PrimitiveComponent Object Reference") (OtherBodyIndex :type Integer) (bFromSweep :type Boolean) (SweepResult :type "HitResult Structure (by ref)"))
  (bind _returnvalue (`self.K2_GetActorLocation`))
  (bind _asbp_base_character (cast `/Game/Programming/Character/BP_Base_Character` OtherActor))
  (`GameplayStatics.ApplyRadialDamage` (`self.BaseDamage`) _returnvalue (`self.DamageRadius`) null (`|MakeArray` (`self.GetOwner` _asbp_base_character)) self (`self.GetInstigatorController`) true)
  (`KismetSystemLibrary.DrawDebugSphere` _returnvalue (`self.DamageRadius`) 12 (struct :`G` 0.022967 :`B` 1.0 :`A` 1.0) 1.0)
  (`GameplayStatics.SpawnEmitterAtLocation` "/Game/Art/Weapons/WeaponEffects/Explosion/P_Explosion.P_Explosion" _returnvalue)
  (`GameplayStatics.PlaySoundAtLocation` "/Engine/EditorSounds/Notifications/CompileFailed.CompileFailed" (0.0 0.0 0.0) (struct) 1.0 1.0 0.0 null null null))

(fn `UserConstructionScript`)