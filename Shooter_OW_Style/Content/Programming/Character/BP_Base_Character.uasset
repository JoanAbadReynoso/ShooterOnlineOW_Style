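; Base character Blueprint that creates crosshair and health indicator widgets for the local player and supports placing claymores.
; Key 1 toggles placement mode, where Tick traces forward from the camera and draws a debug sphere at the impact point.
; Left click spawns BP_Claymoree above that point, yawed from player 0's control rotation, and decrements the remaining count.
; Spawning runs only with authority and has no server RPC; local health prints as debug text.
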(event `self.ReceiveBeginPlay`
  (if (`self.IsLocallyControlled`)
    (`|ExecutionSequence`
      (:`then_0`
        (bind _returnvalue (`|CreateWidget` "/Game/Programming/UI/WBP_Crosshair.WBP_Crosshair_C"))
        (`UserWidget.AddToViewport` _returnvalue 0))
      (:`then_1`
        (bind _returnvalue_2 (`|CreateWidget` "/Game/Materials/UI/WBP_HealthIndicator.WBP_HealthIndicator_C"))
        (`UserWidget.AddToViewport` _returnvalue_2 0)))))

(event `Key|One`
  (params (Key :type "Key Structure"))
  (:`Pressed`
    (`/Engine/EditorBlueprintResources/StandardMacros.FlipFlop`
      (:`A`
        (set `self.ClaymoreAvailable` true))
      (:`B`
        (set `self.ClaymoreAvailable` false)))))

(event `self.ReceiveTick`
  (params (DeltaSeconds :type "Float (single-precision)"))
  (bind _cameracomp (`self.CameraComp`))
  (bind _returnvalue (`SceneComponent.K2_GetComponentLocation` _cameracomp))
  (`|ExecutionSequence`
    (:`then_0`
      (if (`self.ClaymoreAvailable`)
        (bind _outhit (`KismetSystemLibrary.LineTraceSingle` :`Start` _returnvalue :`End` (+ _returnvalue (* (`KismetMathLibrary.GetForwardVector` (`SceneComponent.K2_GetComponentRotation` _cameracomp)) 700.0)) :`TraceChannel` "TraceTypeQuery1" :`TraceColor` (struct :`G` 0.03496 :`B` 1.0 :`A` 1.0)))
        (`KismetSystemLibrary.DrawDebugSphere` (`.ImpactPoint` (`GameplayStatics.BreakHitResult` _outhit)) 100.0 12 (struct :`R` 1.0 :`G` 1.0 :`B` 1.0 :`A` 1.0) (* DeltaSeconds 2.0) 1.0)))
    (:`then_1`
      (if (`self.IsLocallyControlled`)
        (`KismetSystemLibrary.PrintString` (`KismetStringLibrary.Conv_DoubleToString` (`HealthComponent.Health` (`self.HealthComp`))) true true (struct :`G` 0.66 :`B` 1.0 :`A` 1.0) 0.0)))))

(event `Key|LeftMouseButton`
  (params (Key :type "Key Structure"))
  (:`Pressed`
    (`|ExecutionSequence`
      (:`then_0`
        (if (`self.ClaymoreAvailable`)
          (if (> (`self.Claymores Available`) 0)
            (`/Engine/EditorBlueprintResources/ActorMacros.Switch Has Authority`
              (:`Authority`
                (`|SpawnActorFromClass` "/Game/Programming/Actors/Claymore/BP_Claymoree.BP_Claymoree_C" (`KismetMathLibrary.MakeTransform` (`KismetMathLibrary.MakeVector` (.x (`.ImpactPoint` (`GameplayStatics.BreakHitResult` (stale `self.ReceiveTick` _outhit)))) (.y (`.ImpactPoint` (`GameplayStatics.BreakHitResult` (stale `self.ReceiveTick` _outhit)))) (+ (.z (`.ImpactPoint` (`GameplayStatics.BreakHitResult` (stale `self.ReceiveTick` _outhit)))) 40.0)) (`KismetMathLibrary.MakeRotator` 0.0 0.0 (+ (.yaw (`Controller.GetControlRotation` (`GameplayStatics.GetPlayerController` 0))) -80.0)) (0.3 0.3 0.3)) "AdjustIfPossibleButAlwaysSpawn" "OverrideRootScale" null null)
                (bind _result (`/Engine/EditorBlueprintResources/StandardMacros.DecrementInt` (`self.Claymores Available`))
                  (:`  `
                    (`KismetSystemLibrary.PrintString` (`KismetStringLibrary.Conv_IntToString` _result)))))))))))
  (:`Released`
    (set `self.DoAction` false)))

(fn `UserConstructionScript`)