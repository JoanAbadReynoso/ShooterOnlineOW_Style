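; BP_GrenadeLaunced is a grenade ammo actor that explodes on a short fixed timer after spawning, then destroys itself.
; BeginPlay runs the fuse delay and calls the Explode event, which spawns an explosion emitter and applies full, non-falloff radial damage within DamageRadius, credited to the instigator's controller.
; Explode also draws a debug sphere showing the blast radius, and the graph contains no impact or movement logic.
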(event `self.ReceiveBeginPlay`
  (`KismetSystemLibrary.Delay` 1.0)
  (`self.Explode`)
  (`self.K2_DestroyActor`))

(event `Explode`
  (bind _returnvalue (`self.K2_GetActorLocation`))
  (bind _damageradius (`self.DamageRadius`))
  (`GameplayStatics.SpawnEmitterAtLocation` "/Game/Art/Weapons/WeaponEffects/Explosion/P_Explosion.P_Explosion" _returnvalue)
  (`GameplayStatics.ApplyRadialDamage` :`BaseDamage` 100.0 :`Origin` _returnvalue :`DamageRadius` _damageradius :`DamageCauser` self :`InstigatedByController` (`self.GetInstigatorController`) :`bDoFullDamage` true)
  (`KismetSystemLibrary.DrawDebugSphere` _returnvalue _damageradius 12 (struct :`G` 0.150007 :`B` 1.0 :`A` 1.0) 1.0 2.0))

(fn `UserConstructionScript`)